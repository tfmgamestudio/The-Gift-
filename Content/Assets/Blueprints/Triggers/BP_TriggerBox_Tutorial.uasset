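; Trigger box that shows a tutorial message when the BP_TheGiftCharacter player enters it.
; On BeginPlay it creates its own WBP_Tutorial widget, adds it to the viewport and hides it.
; The first overlap, gated by DoOnce, fills in the box's Text variable and shows the widget.
; The message hides after a fixed delay or when the character leaves the box.
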(event `self.ReceiveBeginPlay`
  (bind _returnvalue (`|CreateWidget` "/Game/Assets/Blueprints/UI/WBP_Tutorial.WBP_Tutorial_C" (`GameplayStatics.GetPlayerController` 0)))
  (bind _output_get (set `self.WidgetTutorial` _returnvalue))
  (`UserWidget.AddToViewport` _returnvalue 0)
  (`UserWidget.AddToViewport` _output_get 0)
  (`Widget.SetVisibility` _output_get "Hidden"))

(event `self.CollisionComponent.OnComponentBeginOverlap`
  (params (OverlappedComponent :type "PrimitiveComponent Object Reference") (OtherActor :type "Actor Object Reference") (OtherComp :type "PrimitiveComponent Object Reference") (OtherBodyIndex :type Integer) (bFromSweep :type Boolean) (SweepResult :type "HitResult Structure (by ref)"))
  (bind _widgettutorial (`self.WidgetTutorial`))
  (cast `/Game/Assets/Blueprints/BP_TheGiftCharacter` OtherActor)
  (`/Engine/EditorBlueprintResources/StandardMacros.DoOnce` false
    (:`Completed`
      (`Widget.SetVisibility` _widgettutorial "Visible")
      (set `TextBlock.Text` (`self.Text`) (`/Game/Assets/Blueprints/UI/WBP_Tutorial.TextWidget` _widgettutorial))
      (`KismetSystemLibrary.Delay` 10.0)
      (`Widget.SetVisibility` (`self.WidgetTutorial`) "Hidden"))))

(event `self.CollisionComponent.OnComponentEndOverlap`
  (params (OverlappedComponent :type "PrimitiveComponent Object Reference") (OtherActor :type "Actor Object Reference") (OtherComp :type "PrimitiveComponent Object Reference") (OtherBodyIndex :type Integer))
  (cast `/Game/Assets/Blueprints/BP_TheGiftCharacter` OtherActor)
  (`Widget.SetVisibility` (`self.WidgetTutorial`) "Hidden"))

(fn `UserConstructionScript`)