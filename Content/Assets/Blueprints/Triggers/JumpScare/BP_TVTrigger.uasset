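; BP_TVTrigger is a jump scare trigger volume that can switch on a TV when the player walks into it.
; On box overlap by TheGiftCharacter, a random roll gives a one-in-four chance to fire.
; A successful roll calls TriggerTV on the referenced Remote, but only if the TV is not already on.
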(event `self.Box.OnComponentBeginOverlap`
  (params (OverlappedComponent :type "PrimitiveComponent Object Reference") (OtherActor :type "Actor Object Reference") (OtherComp :type "PrimitiveComponent Object Reference") (OtherBodyIndex :type Integer) (bFromSweep :type Boolean) (SweepResult :type "HitResult Structure (by ref)"))
  (bind _remote (`self.Remote`))
  (bind _asthe_gift_character (cast `TheGiftCharacter` OtherActor))
  (`/Engine/EditorBlueprintResources/StandardMacros.IsValid` _asthe_gift_character
    (:`Is Valid`
      (set `self.RandomInt` (`KismetMathLibrary.RandomIntegerInRange` 0 3))
      (if (== (`self.RandomInt`) 3)
        (if (not (`/Game/Assets/Blueprints/Interactable/BP_TVRemote.IsTVOn` _remote))
          (`/Game/Assets/Blueprints/Interactable/BP_TVRemote.TriggerTV` _remote))))))

(fn `UserConstructionScript`)