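; Player character Blueprint handling footstep audio, a battery-powered flashlight, stamina-limited sprinting and opening the pause menu.
; Tick derives IsMoving from velocity to start or stop the Footsteps audio.
; Looping timers drain the battery while lit and spend or regenerate stamina; sprint requires a minimum stamina, and exhaustion plays a sound and forces walking.
; A temporary RightShift toggle fades a post-process alpha through a Timeline and material parameter collection.
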(event `self.ReceiveTick`
  (params (DeltaSeconds :type "Float (single-precision)"))
  ;[0.05127 0.05127 0.05127] Event Tick
  (`|ExecutionSequence`
    (:`then_0`
      (if (`self.IsMoving`)
        (`/Engine/EditorBlueprintResources/StandardMacros.DoOnce` false :!label _label
          (:`Completed`
            (`AudioComponent.Play` (`self.Footsteps`) 0.0)))
        (else
          (`AudioParameterControllerInterface.SetTriggerParameter` (`self.Footsteps`) "OnStop")
          (`self.ResetFootsteps`))))
    (:`then_1`
      (if (== (`KismetMathLibrary.VSize` (`self.GetVelocity`)) 0.0)
        (set `self.IsMoving` false)
        (else
          (set `self.IsMoving` true))))))

(event `ResetFootsteps`
  ;[0.05127 0.05127 0.05127] Event Tick
  (goto _label :!via `Reset`))

(event `EnhancedInput|/Game/Assets/Input/Actions/IA_Flashlight`
  (params (ActionValue :type Boolean) (ElapsedSeconds :type "Float (double-precision)") (TriggeredSeconds :type "Float (double-precision)") (InputAction :type "InputAction Object Reference" :default "/Game/Assets/Input/Actions/IA_Flashlight.IA_Flashlight"))
  ;[0.05127 0.05127 0.05127] Flashlight Input
  (:`Triggered`
    (`self.ToggleFlashlight`)))

(event `EnhancedInput|/Game/Assets/Input/Actions/IA_Sprint`
  (params (ActionValue :type Boolean) (ElapsedSeconds :type "Float (double-precision)") (TriggeredSeconds :type "Float (double-precision)") (InputAction :type "InputAction Object Reference" :default "/Game/Assets/Input/Actions/IA_Sprint.IA_Sprint"))
  (bind _currentstamina (`self.CurrentStamina`))
  ;[0.05127 0.05127 0.05127] Stamina System
  (:`Triggered`
    (if ActionValue
      ;;[0.03071 0.03071 0.03071] Don't allow sprint if stamina <= 0 or if stamina < 25%
      (if (< _currentstamina 25.0)
        _
        (elif (!= _currentstamina 0.0)
          (`KismetSystemLibrary.K2_ClearAndInvalidateTimerHandle` (`self.StaminaRegenTimerHandle`))
          ;;[0.03071 0.03071 0.03071] Pressed (Sprint)
          (set `CharacterMovementComponent.MaxWalkSpeed` (`self.SprintSpeed`) (`self.CharacterMovement`))
          (bind _returnvalue (`KismetSystemLibrary.K2_SetTimerDelegate` (delegate `UpdateStamina`) (`self.StaminaTimerSpeed`) true))
          (set `self.StaminaSpendTimerHandle` _returnvalue)))
      (else
        ;;[0.03071 0.03071 0.03071] Released (Walk)
        (set `CharacterMovementComponent.MaxWalkSpeed` (`self.WalkSpeed`) (`self.CharacterMovement`) :!label _label_2)
        (`KismetSystemLibrary.K2_ClearAndInvalidateTimerHandle` (`self.StaminaSpendTimerHandle`))
        (if (not (`KismetSystemLibrary.K2_IsValidTimerHandle` (`self.StaminaRegenTimerHandle`)))
          (bind _returnvalue_2 (`KismetSystemLibrary.K2_SetTimerDelegate` (delegate `UpdateStaminaRegen`) (`self.StaminaTimerSpeed`) true))
          (set `self.StaminaRegenTimerHandle` _returnvalue_2))))))

(event `UpdateStamina`
  ;[0.05127 0.05127 0.05127] Stamina System
  ;;[0.03071 0.03071 0.03071] Pressed (Sprint)
  (if (`self.IsMoving`)
    (set `self.CurrentStamina` (`KismetMathLibrary.FClamp` (- (`self.CurrentStamina`) (* (`self.StaminaSpendPerSecond`) (`self.StaminaTimerSpeed`))) 0.0 (`self.MaxStamina`)))
    (if (== (`self.CurrentStamina`) 0.0)
      (`GameplayStatics.PlaySound2D` "/Game/Assets/Sounds/OutOfBreath.OutOfBreath" 1.0 1.0 0.0 null null)
      (`KismetSystemLibrary.K2_ClearAndInvalidateTimerHandle` (`self.StaminaSpendTimerHandle`))
      (`self.RegenStamina`))))

(event `RegenStamina`
  ;[0.05127 0.05127 0.05127] Stamina System
  ;;[0.03071 0.03071 0.03071] Released (Walk)
  (goto _label_2))

(event `UpdateStaminaRegen`
  ;[0.05127 0.05127 0.05127] Stamina System
  ;;[0.03071 0.03071 0.03071] Released (Walk)
  (set `self.CurrentStamina` (`KismetMathLibrary.FClamp` (+ (`self.CurrentStamina`) (* (`self.StaminaRegenPerSecond`) (`self.StaminaTimerSpeed`))) 0.0 (`self.MaxStamina`)))
  (if (== (`self.CurrentStamina`) (`self.MaxStamina`))
    (`KismetSystemLibrary.K2_ClearAndInvalidateTimerHandle` (`self.StaminaRegenTimerHandle`))))

(event `Key|RightShift`
  (params (Key :type "Key Structure"))
  ;[0.05127 0.05127 0.05127] To trigger with event later
  (:`Pressed`
    (`/Engine/EditorBlueprintResources/StandardMacros.FlipFlop`
      (:`A`
        (bind (_direction _newtrack_0) (`Timeline|Timeline` :!label _label_3)
          (:`Update`
            (`KismetMaterialLibrary.SetScalarParameterValue` "/Game/Assets/Materials/PC_PostProcessAlpha.PC_PostProcessAlpha" (`self.AlphaPP`) _newtrack_0))))
      (:`B`
        (goto _label_3 :!via `Reverse`)))))

(event `ActivatePostProcess`
  ;[0.05127 0.05127 0.05127] To trigger with event later
)

(event `EnhancedInput|/Game/Assets/Input/Actions/IA_Pause`
  (params (ActionValue :type Boolean) (ElapsedSeconds :type "Float (double-precision)") (TriggeredSeconds :type "Float (double-precision)") (InputAction :type "InputAction Object Reference" :default "/Game/Assets/Input/Actions/IA_Pause.IA_Pause"))
  (bind _returnvalue (`GameplayStatics.GetPlayerController` 0))
  ;[0.05127 0.05127 0.05127] Pause
  (:`Started`
    (if (not (`self.PauseMenuOpen`))
      (set `self.PauseMenuOpen` true)
      (set `PlayerController.bShowMouseCursor` true _returnvalue)
      (bind _returnvalue_2 (`|CreateWidget` "/Game/Assets/Blueprints/UI/BP_PauseMenu.BP_PauseMenu_C" _returnvalue))
      (bind _output_get (set `self.PauseMenu` _returnvalue_2))
      (`UserWidget.AddToViewport` _output_get 0)
      (`GameplayStatics.SetGamePaused` true)
      (`WidgetBlueprintLibrary.SetInputMode_UIOnlyEx` _returnvalue null)
      (else
        (set `self.PauseMenuOpen` false)
        (`Widget.RemoveFromParent` (`self.PauseMenu`))))))

(fn `FlashlightDepleteBattery`
  (set `self.FlashlightBatteryLevel` (`KismetMathLibrary.FClamp` (- (`self.FlashlightBatteryLevel`) (`self.FlashlightDepletionAmount`)) 0.0 (`self.FlashlightMaxBattery`)))
  (if (<= (`self.FlashlightBatteryLevel`) 0.0)
    (`self.ToggleFlashlight`)))

(fn `ToggleFlashlight`
  (if (not (`self.FlashlightOn`))
    (if (> (`self.FlashlightBatteryLevel`) 0.0)
      (`SceneComponent.SetVisibility` (`self.FlashlighBase`) true true)
      (set `self.FlashlightOn` true)
      (`KismetSystemLibrary.K2_SetTimer` self "FlashlightDepleteBattery" (`self.FlashlightDepletionRate`) true))
    (else
      (`SceneComponent.SetVisibility` (`self.FlashlighBase`) false true)
      (set `self.FlashlightOn` false)
      (`KismetSystemLibrary.K2_ClearTimer` self "FlashlightDepleteBattery"))))

(fn `UserConstructionScript`)