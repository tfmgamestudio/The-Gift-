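; BP_ScareEventFirstFloorDoor is a one-shot jump scare trigger, named for the first-floor door, that fires when the player character overlaps its box.
; It plays an assigned Level Sequence with configurable looping and pause at end.
; Depending on a SoundPoint check, it plays the scare sound at the actor's location after a one-second delay.
; An optional flag then activates the character's post-process effect, which waits for that delay when sound plays.
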(event `self.Box.OnComponentBeginOverlap`
  (params (OverlappedComponent :type "PrimitiveComponent Object Reference") (OtherActor :type "Actor Object Reference") (OtherComp :type "PrimitiveComponent Object Reference") (OtherBodyIndex :type Integer) (bFromSweep :type Boolean) (SweepResult :type "HitResult Structure (by ref)"))
  ;[0.05127 0.05127 0.05127] GenericJumpScare
  (bind _asbp_the_gift_character (cast `/Game/Assets/Blueprints/BP_TheGiftCharacter` OtherActor))
  (`/Engine/EditorBlueprintResources/StandardMacros.IsValid` _asbp_the_gift_character
    (:`Is Valid`
      (`/Engine/EditorBlueprintResources/StandardMacros.DoOnce` false
        (:`Completed`
          ;[0.05127 0.05127 0.05127] Play Sequence
          (bind _outactor (`LevelSequencePlayer.CreateLevelSequencePlayer` (`self.Level Sequence`) (make `MovieSceneSequencePlaybackSettings` false (`self.Loop`) 1.0 0.0 false false false false false false false true)))
          (`MovieSceneSequencePlayer.Play` (`LevelSequenceActor.SequencePlayer` _outactor))
          ;[0.05127 0.05127 0.05127] Play Sound
          (if (not (== (`self.SoundPoint`) null))
            (`KismetSystemLibrary.Delay` 1.0)
            (`GameplayStatics.PlaySoundAtLocation` (`self.JumpscareSound`) (`self.K2_GetActorLocation`) (struct) 1.0 1.0 0.0 null null null null))
          ;[0.05127 0.05127 0.05127] PostProcess
          (if (`self.DoesActivaterPostProcess`)
            (`/Game/Assets/Blueprints/BP_TheGiftCharacter.ActivatePostProcess` _asbp_the_gift_character)))))))

(fn `UserConstructionScript`)