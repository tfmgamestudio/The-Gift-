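; A one-shot trigger, named for an upstairs door scare event, that plays a level sequence when the player character walks into it.
; On box overlap, while enabled, it casts the other actor to TheGiftCharacter and disables itself so it cannot fire again.
; It then creates a player for its LevelSequence variable at runtime, starts playback and prints a debug message.
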(event `self.Box.OnComponentBeginOverlap`
  (params (OverlappedComponent :type "PrimitiveComponent Object Reference") (OtherActor :type "Actor Object Reference") (OtherComp :type "PrimitiveComponent Object Reference") (OtherBodyIndex :type Integer) (bFromSweep :type Boolean) (SweepResult :type "HitResult Structure (by ref)"))
  (if (`self.IsEnabled`)
    (bind _asthe_gift_character (cast `TheGiftCharacter` OtherActor))
    (`/Engine/EditorBlueprintResources/StandardMacros.IsValid` _asthe_gift_character
      (:`Is Valid`
        (set `self.IsEnabled` false)
        (bind _outactor (`LevelSequencePlayer.CreateLevelSequencePlayer` (`self.Level Sequence`) (make `MovieSceneSequencePlaybackSettings` false (struct) 1.0 0.0 false false false false false false false true)))
        (`MovieSceneSequencePlayer.Play` (`LevelSequenceActor.SequencePlayer` _outactor))
        (`KismetSystemLibrary.PrintString` "Play Sequence")))))

(fn `UserConstructionScript`)