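; BP_BatteryPickup is an interactable battery that recharges the player's flashlight in BP_TheGiftCharacter.
; On Interact, it adds BatteryAmount to the flashlight battery level, clamped to the maximum, then destroys itself.
; If the battery is already full, the pickup stays in the world, though CanInteract always returns true.
; The construction script sets the Sphere component's radius from SphereRadius.
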(event `InteractableInterface.Interact`
  ;[0.05127 0.05127 0.05127] Interact Interface
  (bind _asbp_the_gift_character (cast `/Game/Assets/Blueprints/BP_TheGiftCharacter` (`GameplayStatics.GetPlayerCharacter` 0)))
  (bind _output_get (set `self.TheGiftCharacter` _asbp_the_gift_character))
  (bind _flashlightbatterylevel (`/Game/Assets/Blueprints/BP_TheGiftCharacter.FlashlightBatteryLevel` _output_get))
  (bind _flashlightmaxbattery (`/Game/Assets/Blueprints/BP_TheGiftCharacter.FlashlightMaxBattery` _output_get))
  (if (< _flashlightbatterylevel _flashlightmaxbattery)
    (set `/Game/Assets/Blueprints/BP_TheGiftCharacter.FlashlightBatteryLevel` (`KismetMathLibrary.FClamp` (+ _flashlightbatterylevel (`self.BatteryAmount`)) 0.0 _flashlightmaxbattery) (`self.TheGiftCharacter`))
    (`self.K2_DestroyActor`)))

(fn `CanInteract`
  (returns (ReturnValue :type Boolean))
  (return true))

(fn `UserConstructionScript`
  (`SphereComponent.SetSphereRadius` (`self.Sphere`) (`self.Sphere Radius`) true))