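; Trigger volume that plays the game's final jump scare and ending when the player character first overlaps its box.
; It deactivates and locks the final door, kills the flashlight, spawns a monster just behind the player and plays a growl.
; Input, player mesh and HUD are switched off while the view blends to the monster and fades out.
; Timed delays then show the final widget and return to the main menu level.
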(event `self.Box.OnComponentBeginOverlap`
  (params (OverlappedComponent :type "PrimitiveComponent Object Reference") (OtherActor :type "Actor Object Reference") (OtherComp :type "PrimitiveComponent Object Reference") (OtherBodyIndex :type Integer) (bFromSweep :type Boolean) (SweepResult :type "HitResult Structure (by ref)"))
  (bind _returnvalue (`GameplayStatics.GetPlayerCharacter` 0))
  (bind _returnvalue_2 (`GameplayStatics.GetPlayerController` 0))
  (bind _returnvalue_3 (`GameplayStatics.GetPlayerCharacter` 0))
  (bind _finaldoor (`self.FinalDoor`))
  (bind (_returnvalue_location _returnvalue_rotation) (`KismetMathLibrary.BreakTransform` (`self.GetTransform` _returnvalue)))
  ;[0.05127 0.05127 0.05127] GenericJumpScare
  (bind _asbp_the_gift_character (cast `/Game/Assets/Blueprints/BP_TheGiftCharacter` OtherActor))
  (`/Engine/EditorBlueprintResources/StandardMacros.IsValid` _asbp_the_gift_character
    (:`Is Valid`
      (`/Engine/EditorBlueprintResources/StandardMacros.DoOnce` false
        (:`Completed`
          (`InteractableDoorBase.OnDeactivate` _finaldoor)
          (set `InteractableDoorBase.Locked` true _finaldoor)
          (bind _asbp_the_gift_character_2 (cast `/Game/Assets/Blueprints/BP_TheGiftCharacter` _returnvalue))
          (`/Game/Assets/Blueprints/BP_TheGiftCharacter.TurnOffFlashlight` _asbp_the_gift_character_2)
          (bind _returnvalue_4 (`|SpawnActorFromClass` "/Game/Assets/Blueprints/AI/BP_Monster.BP_Monster_C" (`KismetMathLibrary.MakeTransform` (- (`self.K2_GetActorLocation` _returnvalue) (* (`self.GetActorForwardVector` _returnvalue) 50.0)) _returnvalue_rotation) "Undefined" "MultiplyWithRoot" null null))
          (`GameplayStatics.PlaySound2D` "/Game/Assets/Sounds/Jumpscares/SC_MonsterGrowl.SC_MonsterGrowl" 1.0 1.0 0.0 null null)
          (`self.DisableInput` _returnvalue_3 _returnvalue_2)
          (`SceneComponent.SetVisibility` (`Character.Mesh` _returnvalue_3) false false)
          (bind _asthe_gift_player_controller (cast `TheGiftPlayerController` _returnvalue_2))
          (`Widget.SetVisibility` (`TheGiftPlayerController.MainWidget` _asthe_gift_player_controller) "Hidden")
          (`PlayerController.SetViewTargetWithBlend` _returnvalue_2 _returnvalue_4 1.0 "VTBlend_Linear" 0.5 false)
          (`PlayerCameraManager.StartCameraFade` :`self` (`GameplayStatics.GetPlayerCameraManager` 0) :`ToAlpha` 1.0 :`Duration` 3.0 :`bHoldWhenFinished` true)
          (`KismetSystemLibrary.Delay` 3.0)
          (bind _returnvalue_5 (`|CreateWidget` "/Game/Assets/Blueprints/UI/WBP_Final.WBP_Final_C" (`GameplayStatics.GetPlayerController` 0)))
          (`UserWidget.AddToViewport` _returnvalue_5 0)
          (`KismetSystemLibrary.Delay` 10.0)
          (`GameplayStatics.OpenLevel` "L_MainMenu"))))))

(fn `UserConstructionScript`)