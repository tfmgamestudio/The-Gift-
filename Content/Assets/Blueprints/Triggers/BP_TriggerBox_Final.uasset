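; End-of-game trigger box that plays the final scare and ending screen when BP_TheGiftCharacter enters its collision component.
; The overlap activates the character's post-process and plays a monster growl, then after a delay shows the WBP_Final widget and pauses the game.
; A second Delay, issued while paused, precedes opening L_MainMenu and the unpause call.
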(event `self.CollisionComponent.OnComponentBeginOverlap`
  (params (OverlappedComponent :type "PrimitiveComponent Object Reference") (OtherActor :type "Actor Object Reference") (OtherComp :type "PrimitiveComponent Object Reference") (OtherBodyIndex :type Integer) (bFromSweep :type Boolean) (SweepResult :type "HitResult Structure (by ref)"))
  (bind _asbp_the_gift_character (cast `/Game/Assets/Blueprints/BP_TheGiftCharacter` OtherActor))
  (`/Engine/EditorBlueprintResources/StandardMacros.IsValid` _asbp_the_gift_character
    (:`Is Valid`
      (`/Game/Assets/Blueprints/BP_TheGiftCharacter.ActivatePostProcess` _asbp_the_gift_character)
      (`GameplayStatics.PlaySound2D` "/Game/Assets/Sounds/MonsterGrowl.MonsterGrowl" 1.0 1.0 0.0 null null)
      (`KismetSystemLibrary.Delay` 5.0)
      (bind _returnvalue (`|CreateWidget` "/Game/Assets/Blueprints/UI/WBP_Final.WBP_Final_C" (`GameplayStatics.GetPlayerController` 0)))
      (bind _output_get (set `self.Final` _returnvalue))
      (`UserWidget.AddToViewport` _output_get 0)
      (`GameplayStatics.SetGamePaused` true)
      (`KismetSystemLibrary.Delay` 5.0)
      (`GameplayStatics.OpenLevel` "L_MainMenu")
      (`GameplayStatics.SetGamePaused` false))))

(fn `UserConstructionScript`)